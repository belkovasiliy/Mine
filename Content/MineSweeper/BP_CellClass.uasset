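; Minesweeper cell actor that shows its state by swapping textures on a dynamic material instance.
; When the mine character overlaps an unknown cell, it disables that character's input and sends an "open" message with the cell's coordinates to the field manager.
; UpdateCell applies new values, protecting flags except on restart, and mines explode with radial damage and an emitter.
; SetFlag toggles between unknown and flagged.
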(event `self.ReceiveBeginPlay`
  (`KismetSystemLibrary.Delay` 0.0)
  (bind _returnvalue (`PrimitiveComponent.CreateDynamicMaterialInstance` (`self.StaticMesh`) 0 "/Game/MineSweeper/Cell/Materials/M_FalloffNumber_Inst.M_FalloffNumber_Inst" "None"))
  (set `self.Material` _returnvalue)
  (`self.UpdateCell` (`self.CellUnknown`)))

(event `self.StaticMesh.OnComponentBeginOverlap`
  (params (OverlappedComponent :type "PrimitiveComponent Object Reference") (OtherActor :type "Actor Object Reference") (OtherComp :type "PrimitiveComponent Object Reference") (OtherBodyIndex :type Integer) (bFromSweep :type Boolean) (SweepResult :type "HitResult Structure (by ref)"))
  (bind (_celldata_cellx _celldata_celly _celldata_value) (break `CellData` (`self.CellData`)))
  (if (`KismetStringLibrary.EqualEqual_StrStr` _celldata_value (`self.CellUnknown`))
    (bind _asbp_mine_chacracter (cast `/Game/Player/Blueprints/BP_MineChacracter` OtherActor))
    (`/Game/Player/Blueprints/BP_MineChacracter.InputOnOff` _asbp_mine_chacracter false)
    (`self.CheckCell`)))

(event `Restart`
  (bind (_celldata_cellx _celldata_celly) (break `CellData` (`self.CellData`)))
  (set `self.IsRestart` true)
  (set `self.CellData` (make `CellData` _celldata_cellx _celldata_celly (`self.CellUnknown`)))
  (`self.UpdateCell` (`self.CellUnknown`))
  (set `self.IsRestart` false))

(event `CheckCell`
  (bind (_celldata_cellx _celldata_celly) (break `CellData` (`self.CellData`)))
  (bind (_celldata_cellx_2 _celldata_celly_2 _celldata_value) (break `CellData` (`self.CellData`)))
  (if (`KismetStringLibrary.EqualEqual_StrStr` _celldata_value (`self.CellUnknown`))
    (bind _asbp_field_manager_class (cast `/Game/MineSweeper/BP_FieldManagerClass` (`HTBlueprintFunctionLibrary.GetFieldManager`)))
    (`/Game/MineSweeper/BP_FieldManagerClass.SendMessage` _asbp_field_manager_class (`KismetStringLibrary.Concat_StrStr` "open" " " (`KismetStringLibrary.Conv_IntToString` _celldata_cellx) " " (`KismetStringLibrary.Conv_IntToString` _celldata_celly)))))

(event `SetFlag`
  (bind (_celldata_cellx _celldata_celly _celldata_value) (break `CellData` (`self.CellData`)))
  (bind (_celldata_cellx_2 _celldata_celly_2) (break `CellData` (`self.CellData`)))
  (bind _returnvalue (`KismetStringLibrary.EqualEqual_StrStr` _celldata_value (`self.CellFlag`)))
  (bind _returnvalue_2 (`KismetMathLibrary.SelectString` (`self.CellUnknown`) (`self.CellFlag`) _returnvalue))
  (bind (_value _returnvalue_3) (`BlueprintMapLibrary.Map_Find` (`self.CellTextures`) _returnvalue_2))
  (if (or (`KismetStringLibrary.EqualEqual_StrStr` _celldata_value (`self.CellUnknown`)) _returnvalue)
    (if _returnvalue_3
      (`MaterialInstanceDynamic.SetTextureParameterValue` (`self.Material`) "Texture" _value)
      (set `self.CellData` (make `CellData` _celldata_cellx_2 _celldata_celly_2 _returnvalue_2)))))

(fn `UpdateCell`
  (params (StringValue :type String))
  (bind (_celldata_cellx _celldata_celly _celldata_value) (break `CellData` (`self.CellData`)))
  (bind (_celldata_cellx_2 _celldata_celly_2) (break `CellData` (`self.CellData`)))
  (bind (_celldata_cellx_3 _celldata_celly_3 _celldata_value_2) (break `CellData` (`self.CellData`)))
  (bind (_value _returnvalue) (`BlueprintMapLibrary.Map_Find` (`self.CellTextures`) (`local.StringValue`)))
  (bind _returnvalue_2 (`SceneComponent.K2_GetComponentLocation` (`self.StaticMesh`)))
  (`parent.UpdateCell` StringValue)
  (if (`self.IsRestart`)
    (if _returnvalue :!label _label
      (`MaterialInstanceDynamic.SetTextureParameterValue` (`self.Material`) "Texture" _value)
      (set `self.CellData` (make `CellData` _celldata_cellx_2 _celldata_celly_2 (`local.StringValue`)))
      (if (`self.IsRestart`)
        _
        (elif (`KismetStringLibrary.EqualEqual_StrStr` _celldata_value_2 "*")
          (`GameplayStatics.ApplyRadialDamageWithFalloff` :`BaseDamage` 1000.0 :`MinimumDamage` 10.0 :`Origin` _returnvalue_2 :`DamageOuterRadius` 10000.0 :`DamageFalloff` 1.0 :`DamageCauser` null :`InstigatedByController` null :`DamagePreventionChannel` "ECC_Pawn")
          (`GameplayStatics.SpawnEmitterAtLocation` "/Game/Effects/Explosions/Particles/P_ImpactExplosion4.P_ImpactExplosion4" _returnvalue_2))))
    (elif (`KismetStringLibrary.NotEqual_StrStr` _celldata_value "flag")
      (goto _label))))

(fn `UserConstructionScript`
  (`StaticMeshComponent.SetStaticMesh` (`self.StaticMesh`) (`self.StaticMeshRef`)))