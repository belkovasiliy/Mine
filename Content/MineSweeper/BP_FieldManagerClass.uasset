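; Minesweeper field manager that runs the board from a text-based server protocol through BP_HTGameInstance's messaging.
; InitField and Restart request a new field for the current level, with Restart also resetting existing cells.
; Map replies become row characters that build the cell grid on a timer first, then update it.
; Other replies are classified by substring to fire open, lose or victory events, requesting a fresh map except on victory.
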(event `InitField`
  (bind _asbp_htgame_instance (cast `/Game/BP_HTGameInstance` (`GameplayStatics.GetGameInstance`)))
  (if (`/Game/BP_HTGameInstance.IsValidWeb` _asbp_htgame_instance)
    (add `HTGameInstance.OnMessageEvent` _asbp_htgame_instance (`|CreateDelegate` :!event `OnMessageEvent`))
    (`self.SendGenerateField`)))

(event `SendGenerateField`
  (bind _asbp_htgame_instance (cast `/Game/BP_HTGameInstance` (`GameplayStatics.GetGameInstance`)))
  (`self.SendMessage` (`KismetStringLibrary.Concat_StrStr` "new" " " (`KismetStringLibrary.Conv_IntToString` (`/Game/BP_HTGameInstance.LevelNumber` _asbp_htgame_instance)))))

(event `self.ReceiveBeginPlay`)

(event `SendMessage`
  (params (Message :type String))
  (bind _asbp_htgame_instance (cast `/Game/BP_HTGameInstance` (`GameplayStatics.GetGameInstance`)))
  (`/Game/BP_HTGameInstance.SendMessage` _asbp_htgame_instance Message))

(event `OnMessageEvent`
  (params (MessageText :type String))
  (if (`self.Is Update Map Message` MessageText)
    (bind _outarrayrowstring (`self.FormatMessageToRowString` MessageText))
    (set `self.FieldString` _outarrayrowstring)
    (bind _outarrayrowchars (`self.ConvertRowStringToRowChars` (`self.FieldString`)))
    (set `self.ArrayRowChars` _outarrayrowchars)
    (`KismetSystemLibrary.Delay` 0.2)
    (if (`KismetMathLibrary.Conv_IntToBool` (`KismetArrayLibrary.Array_Length` (`self.Cells`)))
      (`self.UpdateField` (`self.ArrayRowChars`) (`self.Cells`))
      (else
        (bind _asbp_cell_class (castclass `/Game/MineSweeper/BP_CellClass` (`self.CellClass`))
          (:`then`
            (bind (_spacer _staticmeshref) (defaults `Object` _asbp_cell_class))
            (set `self.SpawnCellSize` (+ _spacer (* (.x (`.BoxExtent` (`KismetMathLibrary.BreakBoxSphereBounds` (`StaticMesh.GetBounds` _staticmeshref)))) 2.0))))
          (:`CastFailed`
            (set `self.SpawnCellSize` 110.0)))
        (add `self.OnFieldConstructed` (`|CreateDelegate` :!event `OnFieldConstructed_Event`))
        (add `self.OnFieldUpdated` (`|CreateDelegate` :!event `OnFieldUpdated_Event`))
        (`self.ConstructFieldByTimer` (`self.SpawnCellSize`) (`self.ArrayRowChars`) (`self.CountToSpawn`) (`self.SpawnTimeRate`))))
    (else
      (`KismetSystemLibrary.PrintString` MessageText true true (struct :`G` 0.66 :`B` 1.0 :`A` 1.0) 3.0)
      (if (`self.IsOpenCellSuccessMessage` MessageText)
        (`self.OnOpenCellSuccess`)
        (`self.Send Update Field` :!label _label)
        (elif (`self.IsLooseMessage` MessageText)
          (`self.OnLoose`)
          (goto _label)
          (elif (`self.IsWinMessage` MessageText)
            (`self.OnVictory`)
            (else
              (goto _label))))))))

(event `OnFieldUpdated_Event`
  (`KismetSystemLibrary.PrintString` "Updated" true true (struct :`G` 0.66 :`B` 1.0 :`A` 1.0) 5.0))

(event `OnFieldConstructed_Event` :!signature `self.OnFieldConstructed`
  (params (OutCellArray :type "Array of Cell Object Reference (by ref)"))
  (set `self.Cells` OutCellArray)
  (`KismetSystemLibrary.PrintString` (`KismetStringLibrary.Concat_StrStr` "count   " (`KismetStringLibrary.Conv_IntToString` (`KismetArrayLibrary.Array_Length` (`self.Cells`)))) true true (struct :`G` 0.66 :`B` 1.0 :`A` 1.0) 5.0)
  (`KismetSystemLibrary.PrintString` "Constructed" true true (struct :`G` 0.66 :`B` 1.0 :`A` 1.0) 5.0))

(event `Restart`
  ;[1 1 1] Restart
  (for _array_element (`self.Cells`)
    (bind _asbp_cell_class (cast `/Game/MineSweeper/BP_CellClass` _array_element))
    (`/Game/MineSweeper/BP_CellClass.Restart` _asbp_cell_class))
  (`KismetSystemLibrary.Delay` 0.2)
  (`self.SendGenerateField`)
  (`self.OnRestart`))

(fn `Is Update Map Message`
  (params (SourceString :type String))
  (returns (Return :type Boolean))
  (return (and (> (`KismetStringLibrary.FindSubstring` SourceString "map") -1) (not (> (`KismetStringLibrary.FindSubstring` SourceString "help") -1)))))

(fn `IsLooseMessage`
  (params (SourceString :type String))
  (returns (Return :type Boolean))
  (return (and (> (`KismetStringLibrary.FindSubstring` SourceString "You") -1) (> (`KismetStringLibrary.FindSubstring` SourceString "lose") -1))))

(fn `IsOpenCellSuccessMessage`
  (params (SourceString :type String))
  (returns (Return :type Boolean))
  (return (and (> (`KismetStringLibrary.FindSubstring` SourceString "open") -1) (> (`KismetStringLibrary.FindSubstring` SourceString "ok") -1))))

(fn `IsVictoryMessage`
  (params (SourceString :type String))
  (returns (Return :type Boolean))
  (return (and (> (`KismetStringLibrary.FindSubstring` SourceString "new") -1) (not (> (`KismetStringLibrary.FindSubstring` SourceString "help") -1)))))

(fn `IsWinMessage`
  (params (SourceString :type String))
  (returns (Return :type Boolean))
  (return (> (`KismetStringLibrary.FindSubstring` SourceString "win") -1)))

(fn `Send Update Field`
  (`self.SendMessage` "map"))

(fn `UserConstructionScript`)