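; BP_HTGameInstance is a Game Instance Blueprint that owns a WebSocket client connection.
; InitWebSocket creates the socket from a URL when none is valid, binds a connected callback and connects, with short delays and debug prints.
; SendMessage forwards text to the socket, and IsValidWeb reports whether it is valid and connected.
; A handler prints incoming messages, but its binding node is never executed.
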(event `InitWebSocket`
  (if (not (`self.IsValidWebSocket`))
    (`KismetSystemLibrary.Delay` 1.0)
    (`KismetSystemLibrary.PrintString` "Creating")
    (`self.CreateWebSocket` (`self.URL`))
    (add `self.OnConnectedEvent` (delegate `OnConnectedEvent_Event_0`))
    (`KismetSystemLibrary.Delay` 1.0)
    (`KismetSystemLibrary.PrintString` "Connecting")
    (`self.Connect`)))

(event `OnConnectedEvent_Event_0`
  (`KismetSystemLibrary.PrintString` "Connected"))

(event `SendMessage`
  (params (Message :type String))
  (`self.Send` Message))

(event `OnMessageEvent_Event_0` :!signature `self.OnMessageEvent`
  (params (MessageText :type String))
  (`KismetSystemLibrary.PrintString` MessageText true true (struct :`G` 0.66 :`B` 1.0 :`A` 1.0) 100.0))

(fn `IsValidWeb`
  (returns (Valid :type Boolean))
  (if (`self.IsValidWebSocket`)
    (if (`self.IsConnected`)
      (return true)
      (else
        _)))
  (return false))