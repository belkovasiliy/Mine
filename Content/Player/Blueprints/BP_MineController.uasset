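; Player controller that handles the mouse cursor, pause menu and input availability for the player.
; InitController enables mouse events, creates a hidden WBP_Pause and a WBP_Cross cursor widget, and briefly switches to game-only input to force focus before restoring game-and-UI mode.
; SetPause toggles the menu and optionally pauses the game, while UpdateCursor rescales the crosshair on press.
; Input starts disabled at BeginPlay and is switched through InputOnOff.
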(event `self.ReceiveBeginPlay`
  (`self.InputOnOff` false))

(event `InitController`
  (set `self.bEnableMouseOverEvents` true)
  (set `self.bShowMouseCursor` true)
  (set `self.bEnableClickEvents` true)
  (bind _returnvalue (`|CreateWidget` "/Game/Menu/WBP_Pause.WBP_Pause_C" self))
  (bind _output_get (set `self.PauseMenu` _returnvalue))
  (`UserWidget.AddToViewport` _output_get 0)
  (`Widget.SetVisibility` (`self.PauseMenu`) "Collapsed")
  (bind _returnvalue_2 (`|CreateWidget` "/Game/Player/WBP_Cross.WBP_Cross_C" self))
  (bind _output_get_2 (set `self.Cursor` _returnvalue_2))
  (`self.SetMouseCursorWidget` "Default" _output_get_2)
  (`WidgetBlueprintLibrary.SetInputMode_GameOnly` self) ; Forces the mouse/controller to focus on the screen when begin playing
  (`WidgetBlueprintLibrary.SetInputMode_GameAndUIEx` self null "DoNotLock" false) ; Back to normal
)

(event `SetPause`
  (params (PauseGame :type Boolean))
  (switch `ESlateVisibility` (`Widget.GetVisibility` (`self.PauseMenu`))
    (:`Visible`
      (`Widget.SetVisibility` (`self.PauseMenu`) "Collapsed")
      (if (`GameplayStatics.IsGamePaused`)
        (`GameplayStatics.SetGamePaused` false)))
    (:`Collapsed`
      (`Widget.SetVisibility` (`self.PauseMenu`) "Visible" :!label _label)
      (if PauseGame
        (`GameplayStatics.SetGamePaused` true)))
    (:`Hidden`
      (goto _label))))

(event `UpdateCursor`
  (params (Pressed :type Boolean))
  (bind _cursor (`self.Cursor`))
  (bind (_cursorscale_x _cursorscale_y) (`KismetMathLibrary.BreakVector2D` (`self.CursorScale`)))
  (`/Engine/EditorBlueprintResources/StandardMacros.IsValid` _cursor
    (:`Is Valid`
      (`Widget.SetRenderScale` (`/Game/Player/WBP_Cross.T_Cross` _cursor) (select `bool` Pressed :`false` (`KismetMathLibrary.MakeVector2D` _cursorscale_x _cursorscale_x) :`true` (`KismetMathLibrary.MakeVector2D` _cursorscale_y _cursorscale_y))))))

(event `InputOnOff`
  (params (Enable :type Boolean))
  (if Enable
    (`self.EnableInput` self)
    (else
      (`self.DisableInput` self))))

(fn `UserConstructionScript`)