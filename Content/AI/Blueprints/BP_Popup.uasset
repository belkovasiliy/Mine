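; BP_Popup is an actor that follows a SceneLocation component and turns toward the player's camera.
; Each Tick, while SceneLocation is valid, it sets its location and rotation using VInterpTo and RInterpTo with a shared InterpSpeed.
; Rotation eases toward a look-at from SceneLocation to the camera.
; The location interpolation runs from the component toward the actor, so higher speeds make it follow more loosely.
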(event `self.ReceiveTick`
  (params (DeltaSeconds :type "Float (single-precision)"))
  (bind _scenelocation (`self.SceneLocation`))
  (`/Engine/EditorBlueprintResources/StandardMacros.IsValid` _scenelocation
    (:`Is Valid`
      (`self.K2_SetActorLocationAndRotation` (`KismetMathLibrary.VInterpTo` (`SceneComponent.K2_GetComponentLocation` _scenelocation) (`self.K2_GetActorLocation`) DeltaSeconds (`self.InterpSpeed`)) (`KismetMathLibrary.RInterpTo` (`self.K2_GetActorRotation`) (`KismetMathLibrary.FindLookAtRotation` (`SceneComponent.K2_GetComponentLocation` (`self.SceneLocation`)) (`self.K2_GetActorLocation` (`GameplayStatics.GetPlayerCameraManager` 0))) DeltaSeconds (`self.InterpSpeed`))))))

(fn `UserConstructionScript`)