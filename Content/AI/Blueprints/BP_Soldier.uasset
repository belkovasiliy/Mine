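; BP_Soldier is an AI character that reacts to field game events: construction, restart, successful cell opening, loss and victory.
; On BeginPlay it spawns a BP_Popup at SceneLoc and binds to the field manager's events.
; Those events update its state, make it jump or start its AI controller behavior, and show random popup messages looked up by key.
; SetRagdoll toggles mesh physics, restoring the saved relative transform when disabled.
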(event `self.ReceiveBeginPlay`
  (bind _fieldmanager (`self.FieldManager`))
  (set `self.DefaultRelativeTransform` (`SceneComponent.GetRelativeTransform` (`self.Mesh`)))
  (bind _returnvalue (`|SpawnActorFromClass` "/Game/AI/Blueprints/BP_Popup.BP_Popup_C" (`KismetMathLibrary.MakeTransform` (`SceneComponent.K2_GetComponentLocation` (`self.SceneLoc`))) "AlwaysSpawn" "OverrideRootScale" null (`self.SceneLoc`) null))
  (set `self.Popup` _returnvalue)
  (bind _asbp_field_manager_class (cast `/Game/MineSweeper/BP_FieldManagerClass` (`HTBlueprintFunctionLibrary.GetFieldManager`)))
  (set `self.FieldManager` _asbp_field_manager_class)
  (add `FieldManager.OnFieldConstructed` _fieldmanager (delegate `OnFieldConstructed`))
  (add `/Game/MineSweeper/BP_FieldManagerClass.OnRestart` _fieldmanager (delegate `OnRestart_Event_0`))
  (add `/Game/MineSweeper/BP_FieldManagerClass.OnOpenCellSuccess` (`self.FieldManager`) (delegate `OnOpenCellSuccess_Event_1`))
  (add `/Game/MineSweeper/BP_FieldManagerClass.OnLoose` (`self.FieldManager`) (delegate `OnLoose_Event_0`))
  (add `/Game/MineSweeper/BP_FieldManagerClass.OnVictory` (`self.FieldManager`) (delegate `OnVictory_Event_0`)))

(event `OnOpenCellSuccess_Event_1`
  (`self.Jump`)
  (`self.DrawPopup` "Success"))

(event `OnLoose_Event_0`
  (`self.UpdateState` "NewEnumerator3")
  (`self.DrawPopup` "Losing"))

(event `OnVictory_Event_0`
  (`self.UpdateState` "NewEnumerator2")
  (`self.DrawPopup` "Victory"))

(event `OnFieldConstructed`
  (params (OutCellArray :type "Array of Cell Object Reference (by ref)"))
  (`self.DrawPopup` "Construct" 10.0)
  (`self.UpdateState` "NewEnumerator4" :!label _label)
  (bind _asbp_ai_controller (cast `/Game/AI/Blueprints/BP_AI_Controller` (`self.GetController`)))
  (`/Game/AI/Blueprints/BP_AI_Controller.InitBehavior` _asbp_ai_controller))

(event `OnRestart_Event_0`
  (`self.DrawPopup` "Restart")
  (goto _label))

(event `UpdateState`
  (params (State :type "/Game/AI/SkeletalMesh/E_AnimState Enum" :default "NewEnumerator0"))
  (set `self.State` State))

(event `SetRagdoll`
  (params (Enable :type Boolean))
  (bind _mesh (`self.Mesh`))
  (bind _mesh_2 (`self.Mesh`))
  (if Enable
    (`PrimitiveComponent.SetCollisionProfileName` _mesh "PhysicsActor" false)
    (`PrimitiveComponent.SetSimulatePhysics` _mesh true)
    (else
      (`PrimitiveComponent.SetSimulatePhysics` _mesh_2 false)
      (`PrimitiveComponent.SetCollisionProfileName` _mesh_2 "CharacterMesh" false)
      (`SceneComponent.K2_AttachToComponent` (`self.Mesh`) (`self.CapsuleComponent`) "None" "SnapToTarget" "SnapToTarget" "KeepWorld" true)
      (`SceneComponent.K2_SetRelativeTransform` (`self.Mesh`) (`self.DefaultRelativeTransform`) false false))))

(event `DrawPopup`
  (params (Key :type String) (DrawTime :type "Float (double-precision)" :default 5.0))
  (bind (_value _returnvalue) (`BlueprintMapLibrary.Map_Find` (`self.Messages`) Key))
  (if _returnvalue
    (bind _asui_hint_message (cast `/Game/AI/Hint/UI_HintMessage` (`WidgetComponent.GetUserWidgetObject` (`/Game/AI/Blueprints/BP_Popup.Widget` (`self.Popup`)))))
    (`/Game/AI/Hint/UI_HintMessage.DrawPopup` _asui_hint_message (`|GetArrayItem` (break `/Game/AI/Hint/S_PopupMessage` _value) (`KismetMathLibrary.RandomIntegerInRange` 0 (`KismetArrayLibrary.Array_LastIndex` (break `/Game/AI/Hint/S_PopupMessage` _value)))) DrawTime)))

(fn `UserConstructionScript`)